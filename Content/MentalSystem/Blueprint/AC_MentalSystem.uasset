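; Actor component that tracks a Mental value, with functions for damage, gain and timed recovery.
; Damage subtracts without clamping and calls OnMentalZero only when the value is already exactly zero on entry; gain caps at MaxMental.
; RecoverMental starts a looping one-second timer adding RecoveryRate within bounds, plus a second timer that stops it after the given duration.
; Debug prints report changes, and EventGraph holds only unconnected leftover timer logic.
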(event `_StopGenerate`
  (`KismetSystemLibrary.K2_ClearAndInvalidateTimerHandle` (stale `_StartGenerate` _returnvalue)))

(event `_StartGenerate`
  (params (DeltaTime :type "Float (double-precision)"))
  (`KismetSystemLibrary.K2_SetTimerDelegate` (delegate `_StopGenerate`) DeltaTime)
  (bind _returnvalue (`KismetSystemLibrary.K2_SetTimerDelegate` (delegate `_RegenerateMental`) 1.0 true)))

(event `_RegenerateMental`
  (bind _output_get (set `self.CurrentMental` (`KismetMathLibrary.FClamp` (+ (`self.CurrentMental`) (`self.RecoveryRate`)) 0.0 (`self.MaxMental`))))
  (`KismetSystemLibrary.PrintText` (`|FormatText` "recover: {value}" _output_get)))

(fn `ApplyMentalDamage`
  (params (Value :type "Float (double-precision)") (Type :type "/Game/MentalSystem/enum/E_MentalInfluenceType Enum" :default "NewEnumerator0") (Source :type "Actor Object Reference"))
  (if (== (`self.CurrentMental`) 0.0)
    (`self.OnMentalZero`)
    (else
      (set `self.CurrentMental` (- (`self.CurrentMental`) Value))))
  (`KismetSystemLibrary.PrintText` (`|FormatText` "Current Mental: {mentalValue}. {type} Damage from {source}" (`self.CurrentMental`) Source (`|GenericToText` Type))))

(fn `ApplyMentalGain`
  (params (Value :type "Float (double-precision)") (Type :type "/Game/MentalSystem/enum/E_MentalInfluenceType Enum" :default "NewEnumerator0") (Source :type "Actor Object Reference"))
  (bind _returnvalue (+ (`self.CurrentMental`) Value))
  (if (< (`self.CurrentMental`) (`self.MaxMental`))
    (if (>= _returnvalue (`self.MaxMental`))
      (set `self.CurrentMental` (`self.MaxMental`))
      (else
        (set `self.CurrentMental` _returnvalue)))
    (`KismetSystemLibrary.PrintText` (`|FormatText` "Current Mental: {mentalValue}. {type} Gain from {source}" (`self.CurrentMental`) (`|GenericToText` Type) Source))))

(fn `RecoverMental`
  (params (DeltaTime :type "Float (double-precision)"))
  (`KismetSystemLibrary.PrintString` "regen")
  (`self._StartGenerate` DeltaTime))