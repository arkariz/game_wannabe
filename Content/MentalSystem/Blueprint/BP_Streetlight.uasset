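; BP_Streetlight is a streetlight actor that applies a mental influence to an actor overlapping its box.
; Begin overlap starts a one-second looping timer that messages the overlapping actor with influence value, type and source; end overlap clears it.
; Its getter functions supply a fixed value, a fixed type and itself as source.
; The sequence fetches type and source after sending the message, so the first send precedes those calls.
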(event `self.Box.OnComponentEndOverlap`
  (params (OverlappedComponent :type "PrimitiveComponent Object Reference") (OtherActor :type "Actor Object Reference") (OtherComp :type "PrimitiveComponent Object Reference") (OtherBodyIndex :type Integer))
  (`KismetSystemLibrary.K2_ClearAndInvalidateTimerHandle` (stale `self.Box.OnComponentBeginOverlap` _returnvalue)))

(event `self.Box.OnComponentBeginOverlap`
  (params (OverlappedComponent :type "PrimitiveComponent Object Reference") (OtherActor :type "Actor Object Reference") (OtherComp :type "PrimitiveComponent Object Reference") (OtherBodyIndex :type Integer) (bFromSweep :type Boolean) (SweepResult :type "HitResult Structure (by ref)"))
  (bind _returnvalue (`KismetSystemLibrary.K2_SetTimerDelegate` (delegate `ApplyMentalEffect`) 1.0 true)))

(event `ApplyMentalEffect`
  (`|ExecutionSequence`
    (:`then_0`
      (bind _value (`self.GetInfluenceValue`))
      (message `/Game/MentalSystem/BlueprintInterface/BPI_MentalReceiver.ApplyMentalEffect` (stale `self.Box.OnComponentBeginOverlap` OtherActor) _value (stale _type) (stale _actor)))
    (:`then_1`
      (bind _type (`self.GetInfluenceType`)))
    (:`then_2`
      (bind _actor (`self.GetInfluenceSourceActor`)))))

(fn `GetInfluenceSourceActor`
  (returns (Actor :type "Actor Object Reference"))
  (return self))

(fn `GetInfluenceType`
  (returns (Type :type "/Game/MentalSystem/enum/E_MentalInfluenceType Enum"))
  (return "NewEnumerator3"))

(fn `GetInfluenceValue`
  (returns (value :type "Float (double-precision)"))
  (return 15.0))

(fn `UserConstructionScript`)