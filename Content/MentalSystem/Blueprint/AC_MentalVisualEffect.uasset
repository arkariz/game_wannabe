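; Actor component that drives post-process visuals for a character's mental state, from Stable through Unstable and Distorted to Breakdown.
; SetMentalVisualEffect maps each state to target vignette, saturation and contrast, growing darker-edged, greyer and flatter as the state worsens.
; Tick eases current values toward those targets with FInterpTo at BlendSpeed and rebuilds the settings on the owner's PostProcessComponent, found at BeginPlay.
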(event `self.ReceiveBeginPlay`
  (set `self.PostProcessComp` (`Actor.GetComponentByClass` (`self.GetOwner`) "/Script/Engine.PostProcessComponent")))

(event `self.ReceiveTick`
  (params (DeltaSeconds :type "Float (single-precision)"))
  (`|ExecutionSequence`
    (:`then_0`
      (bind _output_get (set `self.CurrentVignette` (`KismetMathLibrary.FInterpTo` (`self.CurrentVignette`) (`self.TargetVignette`) DeltaSeconds (`self.BlendSpeed`))))
      (set `PostProcessComponent.Settings` (make `PostProcessSettings` :`ColorSaturation` (`KismetMathLibrary.MakeVector4` (stale _output_get_2) (stale _output_get_2) (stale _output_get_2) 1.0) :`ColorContrast` (`KismetMathLibrary.MakeVector4` (stale _output_get_3) (stale _output_get_3) (stale _output_get_3) 1.0) :`VignetteIntensity` _output_get) (`self.PostProcessComp`)))
    (:`then_1`
      (bind _output_get_2 (set `self.CurrentSaturation` (`KismetMathLibrary.FInterpTo` (`self.CurrentSaturation`) (`self.TargetSaturation`) DeltaSeconds (`self.BlendSpeed`)))))
    (:`then_2`
      (bind _output_get_3 (set `self.CurrentContrast` (`KismetMathLibrary.FInterpTo` (`self.CurrentContrast`) (`self.TargetContrast`) DeltaSeconds (`self.BlendSpeed`)))))))

(fn `_SetBreakdown`
  (`|ExecutionSequence`
    (:`then_0`
      (set `self.TargetVignette` 1.0))
    (:`then_1`
      (set `self.TargetSaturation` 0.4))
    (:`then_2`
      (set `self.TargetContrast` 0.85))))

(fn `_SetDistorted`
  (`|ExecutionSequence`
    (:`then_0`
      (set `self.TargetVignette` 0.75))
    (:`then_1`
      (set `self.TargetSaturation` 0.6))
    (:`then_2`
      (set `self.TargetContrast` 0.9))))

(fn `_SetStable`
  (`|ExecutionSequence`
    (:`then_0`
      (set `self.TargetVignette` 0.1))
    (:`then_1`
      (set `self.TargetSaturation` 1.0))
    (:`then_2`
      (set `self.TargetContrast` 1.0))))

(fn `_SetUnstable`
  (`|ExecutionSequence`
    (:`then_0`
      (set `self.TargetVignette` 0.5))
    (:`then_1`
      (set `self.TargetSaturation` 0.8))
    (:`then_2`
      (set `self.TargetContrast` 0.95))))

(fn `SetMentalVisualEffect`
  (params (MentalState :type "/Game/MentalSystem/enum/E_MentalState Enum" :default "NewEnumerator0"))
  (switch `/Game/MentalSystem/enum/E_MentalState` MentalState
    (:`NewEnumerator0`
      (`self._SetStable`))
    (:`NewEnumerator1`
      (`self._SetUnstable`))
    (:`NewEnumerator2`
      (`self._SetDistorted`))
    (:`NewEnumerator4`
      (`self._SetBreakdown`))))